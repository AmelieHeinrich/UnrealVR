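; BP_VRButton is a pressable button in the climbing game that starts the VR player's watch timer.
; When a VRPawn overlaps its box, it calls StartWatchTimer on the pawn every time, even while already pressed.
; If not already active, it sinks the button cube and runs a 20-second timer, after which the cube rises and the button re-arms.
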(event `self.Box.OnComponentBeginOverlap`
  (params (OverlappedComponent :type "PrimitiveComponent Object Reference") (OtherActor :type "Actor Object Reference") (OtherComp :type "PrimitiveComponent Object Reference") (OtherBodyIndex :type Integer) (bFromSweep :type Boolean) (SweepResult :type "HitResult Structure (by ref)"))
  (bind _asvrpawn (cast `/Game/VRTemplate/Blueprints/VRPawn` OtherActor))
  (`/Game/VRTemplate/Blueprints/VRPawn.StartWatchTimer` _asvrpawn)
  (if (not (`self.bIsTimerActive`))
    (`KismetSystemLibrary.K2_SetTimerDelegate` (delegate `OnTimerFinished`) 20.0)
    (set `self.bIsTimerActive` true)
    (`SceneComponent.K2_AddWorldOffset` (`self.ButtonCube`) (0.0 0.0 -15.0) true false)))

(event `OnTimerFinished`
  (set `self.bIsTimerActive` false)
  (`SceneComponent.K2_AddWorldOffset` (`self.ButtonCube`) (0.0 0.0 15.0) true false))

(fn `UserConstructionScript`)
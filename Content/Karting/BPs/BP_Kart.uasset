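; BP_Kart is a VR kart that the player mounts and dismounts with the left shoot input, toggling seat attachment and teleporting.
; Each tick, the left hand's angle in kart space, amplified and clamped, rolls the steering wheel and sets the yaw rate.
; While seated, the kart moves forward at constant speed by world offset, but steering applies even unseated.
; Mounting has no proximity check, and GrabDetection is an unfinished stub.
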(event `self.ReceiveBeginPlay`
  (bind _asvrpawn (cast `/Game/VRTemplate/Blueprints/VRPawn` (`GameplayStatics.GetPlayerPawn` 0)))
  (set `self.As VRPawn` _asvrpawn)
  (set `self.debug_lefthand_location_start` (`SceneComponent.K2_GetComponentLocation` (`/Game/VRTemplate/Blueprints/VRPawn.HandLeft` _asvrpawn))))

(event `self.ReceiveTick`
  (params (DeltaSeconds :type "Float (single-precision)"))
  (bind _returnvalue (`KismetMathLibrary.ClampAngle` (* (`KismetMathLibrary.DegAtan2` (.y (`KismetMathLibrary.InverseTransformLocation` (`SceneComponent.K2_GetComponentToWorld` (`self.DefaultSceneRoot`)) (`SceneComponent.K2_GetComponentLocation` (`/Game/VRTemplate/Blueprints/VRPawn.HandLeft` (`self.As VRPawn`))))) (.z (`KismetMathLibrary.InverseTransformLocation` (`SceneComponent.K2_GetComponentToWorld` (`self.DefaultSceneRoot`)) (`SceneComponent.K2_GetComponentLocation` (`/Game/VRTemplate/Blueprints/VRPawn.HandLeft` (`self.As VRPawn`)))))) 6.0) -170.0 -10.0))
  (`|ExecutionSequence`
    (:`then_0`
      (`SceneComponent.K2_SetRelativeRotation` (`self.SteeringWheel`) (`KismetMathLibrary.MakeRotator` _returnvalue) false false))
    (:`then_1`
      (if (`self.IsSeated`)
        (`self.K2_AddActorWorldOffset` (* (* (`self.GetActorForwardVector`) 500.0) (`GameplayStatics.GetWorldDeltaSeconds`)))))
    (:`then_2`
      (`self.K2_AddActorLocalRotation` (`KismetMathLibrary.MakeRotator` 0.0 0.0 (* (* (`KismetMathLibrary.MapRangeClamped` _returnvalue -170.0 -10.0 -100.0 100.0) 2.0) (`GameplayStatics.GetWorldDeltaSeconds`)))))))

(event `EnhancedInput|/Game/VRTemplate/Input/Actions/IA_Shoot_Left`
  (params (ActionValue :type Boolean) (ElapsedSeconds :type "Float (double-precision)") (TriggeredSeconds :type "Float (double-precision)") (InputAction :type "InputAction Object Reference" :default "/Game/VRTemplate/Input/Actions/IA_Shoot_Left.IA_Shoot_Left"))
  (bind _as_vrpawn (`self.As VRPawn`))
  (:`Triggered`
    (if (`self.IsSeated`)
      (`KismetSystemLibrary.PrintString` "Dismounting;;;")
      (`self.K2_DetachFromActor` _as_vrpawn "KeepWorld" "KeepWorld" "KeepWorld")
      (`self.K2_SetActorLocationAndRotation` :`self` _as_vrpawn :`NewLocation` (`SceneComponent.K2_GetComponentLocation` (`self.ExitAnchor`)))
      (set `self.IsSeated` false)
      (set `/Game/VRTemplate/Blueprints/VRPawn.CanTP` true _as_vrpawn)
      (else
        (set `/Game/VRTemplate/Blueprints/VRPawn.CanTP` false _as_vrpawn)
        (`KismetSystemLibrary.PrintString` "Mounting...")
        (`self.K2_AttachToComponent` _as_vrpawn (`self.SeatAnchor`) "None" "SnapToTarget" "SnapToTarget" "KeepWorld" false)
        (set `self.IsSeated` true)))))

(fn `GrabDetection`
  (params (HandComponent :type "MotionControllerComponent Object Reference") (isGrabbed :type Boolean))
  (set `self.Hand Component` HandComponent))

(fn `UserConstructionScript`)
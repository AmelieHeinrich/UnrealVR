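; BP_CubeSpawner is an actor that produces a continuous stream of BP_Cube actors, one spawn at BeginPlay and another whenever a cube stops overlapping its Box component.
; Each spawn waits a short Delay, then places the cube at the Box transform with a random sideways and vertical offset.
; The new cube randomly receives one of two types through SetCubeType.
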(event `self.ReceiveBeginPlay`
  (`self.SpawnCube`))

(event `self.Box.OnComponentEndOverlap`
  (params (OverlappedComponent :type "PrimitiveComponent Object Reference") (OtherActor :type "Actor Object Reference") (OtherComp :type "PrimitiveComponent Object Reference") (OtherBodyIndex :type Integer))
  (if (`.bSuccess` (cast `/Game/Saber/BP_Cube` OtherActor :!pure true))
    (`self.SpawnCube`)))

(event `SpawnCube`
  (bind (_returnvalue_location _returnvalue_rotation _returnvalue_scale) (`KismetMathLibrary.BreakTransform` (`SceneComponent.K2_GetComponentToWorld` (`self.Box`))))
  (`KismetSystemLibrary.Delay` 0.5)
  (bind _returnvalue (`|SpawnActorFromClass` "/Game/Saber/BP_Cube.BP_Cube_C" (`KismetMathLibrary.MakeTransform` (+ _returnvalue_location (`KismetMathLibrary.MakeVector` (`KismetMathLibrary.RandomFloatInRange` 0.0) (`KismetMathLibrary.RandomFloatInRange` -510.0 510.0) (`KismetMathLibrary.RandomFloatInRange` -65.0 65.0))) _returnvalue_rotation _returnvalue_scale) "Undefined" "MultiplyWithRoot" null null))
  (`/Game/Saber/BP_Cube.Set Cube Type` _returnvalue (`KismetMathLibrary.RandomIntegerInRange` 0 1)))

(fn `UserConstructionScript`)
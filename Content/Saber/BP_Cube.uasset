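; BP_Cube is a typed, colored target for a VR saber game that travels along negative world X a fixed step each tick.
; SetCubeType stores the type and tints a dynamic material's emissive color from SaberColors.
; When its Box overlaps a BP_Saber, it triggers controller rumble and compares types.
; RequestDestroy adds a point to every VRPawn for a match or subtracts one for a mismatch, then destroys the cube.
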(event OnComponentBeginOverlap(Box)
  (params (OverlappedComponent :type Primitive%20Component%20Object%20Reference) (OtherActor :type Actor%20Object%20Reference) (OtherComp :type Primitive%20Component%20Object%20Reference) (OtherBodyIndex :type Integer) (bFromSweep :type Boolean) (SweepResult :type Hit%20Result%20Structure%20%28by%20ref%29))
  (bind _asbp_saber (Utilities|Casting|CastToBP_Saber OtherActor))
  (Game|Feedback|PlayDynamicForceFeedback (Game|GetPlayerController 0) 1.0 0.1 true true true true)
  (if (stale _bsuccess)
    (if (== (Variables|/Game/Saber/BP_Saber.BP_Saber_C|GetType _asbp_saber) (Variables|Default|GetType))
      (CallFunction|RequestDestroy true)
      (else
        (CallFunction|RequestDestroy false)))))

(event Custom|Request%20Destroy
  (params (Hit%20by%20saber :type Boolean))
  (Utilities|FlowControl|Sequence
    (:then_0
      (if Hit%20by%20saber
        (bind _outactors (Actor|GetAllActorsOfClass "/Game/VRTemplate/Blueprints/VRPawn.VRPawn_C"))
        (for _array_element _outactors
          (Default|UpdateScore _array_element 1))
        (Actor|DestroyActor)
        (else
          (bind _outactors_2 (Actor|GetAllActorsOfClass "/Game/VRTemplate/Blueprints/VRPawn.VRPawn_C"))
          (for _array_element_2 _outactors_2
            (Default|UpdateScore _array_element_2 -1))
          (Actor|DestroyActor))))
    (:then_1
      (Actor|DestroyActor))))

(event EventBeginPlay)

(event Collision|EventActorBeginOverlap
  (params (OtherActor :type Actor%20Object%20Reference)))

(event EventTick
  (params (DeltaSeconds :type Float%20%28single-precision%29))
  (bind _cube (Variables|Default|GetCube))
  (Transformation|SetWorldLocation _cube (- (Transformation|GetWorldLocation _cube) (Math|Vector|MakeVector 1e+01 0.0 0.0)) false false))

(fn ConstructionScript)

(fn SetCubeType
  (params (Type :type Integer))
  (bind _returnvalue (Rendering|Material|CreateDynamicMaterialInstance (Variables|Default|GetCube) 0 "/Game/Saber/M_Cube.M_Cube" "" :!class /Script/Engine.PrimitiveComponent))
  (Rendering|Material|SetVectorParameterValue _returnvalue "EmissiveColor" (Utilities|Array|Get(acopy) (Variables|Default|GetSaber_Colors) Type) :!class /Script/Engine.MaterialInstanceDynamic)
  (Variables|Default|SetType Type))